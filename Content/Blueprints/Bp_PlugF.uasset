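; Bp_PlugF is a socket that detects and snaps in a nearby Bp_PlugM plug.
; A fast looping timer started on BeginPlay runs a sphere trace at the socket, using DetectionRadius.
; When it hits a plug that is not held, it stores the reference both ways, matches the plug to its own transform and pauses the timer.
; Unplug clears its plug reference and resumes detection.
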(event `self.ReceiveBeginPlay`
  (bind _returnvalue (`KismetSystemLibrary.K2_SetTimerDelegate` (delegate `Test for Plug`) 0.01 true))
  (set `self.Plug Check` _returnvalue))

(event `Test for Plug`
  (bind _returnvalue (`self.K2_GetComponentLocation`))
  (bind _outhit (`KismetSystemLibrary.SphereTraceSingle` _returnvalue (+ _returnvalue 1) (`self.Detection Radius`) "TraceTypeQuery3"))
  (bind (_bblockinghit _binitialoverlap _time _distance _location _impactpoint _normal _impactnormal _physmat _hitactor) (`GameplayStatics.BreakHitResult` _outhit))
  (if _bblockinghit
    (bind _asbp_plug_m (cast `/Game/Blueprints/Bp_PlugM` _hitactor))
    (if (not (`/Game/Blueprints/Bp_PlugM.Held` _asbp_plug_m))
      (bind _output_get (set `self.Plug` _asbp_plug_m))
      (set `/Game/Blueprints/Bp_PlugM.Socket` self _output_get)
      (`Actor.K2_SetActorLocation` _output_get (`self.K2_GetComponentLocation`) false false)
      (`Actor.K2_SetActorRotation` _output_get (`self.K2_GetComponentRotation`) false)
      (`KismetSystemLibrary.K2_PauseTimerHandle` (`self.Plug Check`)))))

(event `Unplug`
  (set `self.Plug` null)
  (`KismetSystemLibrary.K2_UnPauseTimerHandle` (`self.Plug Check`)))